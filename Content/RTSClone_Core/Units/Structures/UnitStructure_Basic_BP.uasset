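; Basic structure unit for the RTS that builds its appearance from static unit data when set up.
; After the parent setup, it synchronously loads the configured mesh, positions it by the placement ghost offset in 50-unit steps, and optionally adds a dev platform mesh.
; It then gives each static mesh component a dynamic material on slot 0, tinted with the owning player's team color from the multiplayer game state.
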(fn `SetupUnit`
  (params (StaticData :type "UnitData_Static Object Reference") (Controller :type "Controller Object Reference"))
  (returns (ReturnValue :type Boolean))
  (bind ((`MeshToUse` _meshtouse) (`Transform` _transform) (`AddPlatform` _addplatform) (`PlacementGhostOffset` _placementghostoffset)) (break `UnitData_StaticStruct` (`UnitData_Static.UnitData_Static` StaticData)))
  (bind (_x _y) (`KismetMathLibrary.BreakVector2D` _placementghostoffset))
  (bind _rotation (.rotation _transform))
  (bind _returnvalue (`KismetMathLibrary.MakeVector` (* _x 50.0) (* _y 50.0)))
  (`parent.SetupUnit` StaticData Controller)
  (`KismetSystemLibrary.PrintString` "Setting up unit...")
  (`|ExecutionSequence`
    (:`then_0`
      (bind _returnvalue_2 (`KismetSystemLibrary.LoadAsset_Blocking` _meshtouse))
      (bind _asstatic_mesh (cast `StaticMesh` _returnvalue_2))
      (`StaticMeshComponent.SetStaticMesh` (`self.StaticMesh`) _asstatic_mesh)
      (`SceneComponent.K2_SetRelativeLocationAndRotation` (`self.StaticMesh`) _returnvalue _rotation false false)
      (if _addplatform
        (bind _returnvalue_3 (`AddComponent|NODE_AddStaticMeshComponent-1` :`RelativeTransform` (`KismetMathLibrary.MakeTransform` _returnvalue _rotation)))
        (`StaticMeshComponent.SetStaticMesh` _returnvalue_3 "/Game/DeveloperLibrary/Meshes/SM_DevPlatform.SM_DevPlatform")))
    (:`then_1`
      (bind _asrtsgame_state_multiplayer_bp (cast `/Game/RTSClone_Core/Game/RTSGameState_Multiplayer_BP` (`GameplayStatics.GetGameState`)))
      (for _array_element (`self.K2_GetComponentsByClass` "/Script/Engine.StaticMeshComponent")
        (bind _returnvalue_4 (`PrimitiveComponent.CreateDynamicMaterialInstance` _array_element 0 (`PrimitiveComponent.GetMaterial` _array_element 0) "None"))
        (`PrimitiveComponent.SetMaterial` _array_element 0 _returnvalue_4)
        (`MaterialInstanceDynamic.SetVectorParameterValue` _returnvalue_4 "Color" (`KismetMathLibrary.Conv_ColorToLinearColor` (`RTSGameState_Multiplayer.GetTeamColorFromController` _asrtsgame_state_multiplayer_bp (`UnitInterface.GetOwningPlayer`))))))
    (:`then_2`
      (return true))))

(fn `UserConstructionScript`)